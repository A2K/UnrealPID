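; Helicopter pawn whose orthographic camera zooms to fit the largest PID value among actors in the level.
; Each tick it scans all actors of the Object class for the greatest absolute current value on their valid PID references.
; That maximum is scaled, floored at a base ortho width and multiplied by the camera's aspect ratio to set the ortho width.
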(event `self.ReceiveTick`
  (params (DeltaSeconds :type "Float (single-precision)"))
  (`self.UpdateCameraWidth`))

(fn `GetMaxObjectValue`
  (returns (Value :type "Float (double-precision)"))
  (locals (MaxValue :type "Float (double-precision)"))
  (`|ExecutionSequence`
    (:`then_0`
      (set `local.MaxValue` 0.0))
    (:`then_1`
      (bind _outactors (`GameplayStatics.GetAllActorsOfClass` "/Game/Object.Object_C"))
      (for _array_element _outactors
        (bind _pid (`/Game/Object.PID` _array_element))
        (`/Engine/EditorBlueprintResources/StandardMacros.IsValid` _pid
          (:`Is Valid`
            (bind _returnvalue (`KismetMathLibrary.Abs` (`/Game/PID.CurrentValue` _pid)))
            (if (> _returnvalue (`local.MaxValue`))
              (set `local.MaxValue` _returnvalue))))))
    (:`then_2`
      (return (`local.MaxValue`)))))

(fn `UpdateCameraWidth`
  (bind _value (`self.GetMaxObjectValue`))
  (`CameraComponent.SetOrthoWidth` (`self.Camera`) (* (`KismetMathLibrary.FMax` (* _value 200.0) (`self.BaseOrthoWidth`)) (`CameraComponent.AspectRatio` (`self.Camera`)))))

(fn `UserConstructionScript`)