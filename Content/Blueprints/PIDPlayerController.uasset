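; Player controller for a helicopter game with PID setpoint control and a game-and-UI input mode.
; Mouse buttons fire the first Helicopter's weapons; number keys repair it, damage it or buy rockets with HUD coins.
; CoordinatePlane click events pass a setpoint to the HUD and actors' PID components.
; Tick can re-trigger clicks from the cursor trace, but the logic enabling ChangingSetpoint is disconnected.
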(event `self.ReceiveBeginPlay`
  (`KismetSystemLibrary.Delay` 0.2)
  (`WidgetBlueprintLibrary.SetInputMode_GameAndUIEx` self (`/Game/Blueprints/PIDHUD.PIDWidget` (`self.HUD`)) "DoNotLock" false)
  (bind _outactors (`GameplayStatics.GetAllActorsOfClass` "/Game/Blueprints/CoordinatePlane.CoordinatePlane_C"))
  (if (> (`KismetArrayLibrary.Array_Length` _outactors) 0)
    (add `/Game/Blueprints/CoordinatePlane.Clicked` (`|GetArrayItem` _outactors) (delegate `OnCoordinatePlaneClicked`))))

(event `OnCoordinatePlaneClicked`
  (params (Location :type "Vector2D Structure"))
  (bind _output_get (set `self.Setpoint` Location_Y))
  (`/Game/Blueprints/PIDHUD.SetSetpoint` (`self.HUD`) _output_get)
  (bind _outactors (`GameplayStatics.GetAllActorsOfClass` "/Game/Object.Object_C"))
  (for _array_element _outactors
    (bind _pid (`/Game/Object.PID` _array_element))
    (`/Engine/EditorBlueprintResources/StandardMacros.IsValid` _pid
      (:`Is Valid`
        (set `/Game/PID.Setpoint` _output_get _pid)))))

(event `self.ReceiveTick`
  (params (DeltaSeconds :type "Float (single-precision)"))
  (bind (_bblockinghit _binitialoverlap _time _distance _location _impactpoint _normal _impactnormal _physmat _hitactor) (`GameplayStatics.BreakHitResult` (`self.GetHitResultUnderCursorForObjects` (`|MakeArray` "ObjectTypeQuery1" "ObjectTypeQuery2" :!type "EObjectTypeQuery Enum") false)))
  (`|ExecutionSequence`
    (:`then_1`
      (if (`self.ChangingSetpoint`)
        (bind _ascoordinate_plane (cast `/Game/Blueprints/CoordinatePlane` _hitactor))
        (`/Game/Blueprints/CoordinatePlane.Clicked` _ascoordinate_plane (`KismetMathLibrary.MakeVector2D` (.y (/ _location 100.0)) (.z (/ _location 100.0))))))))

(event `Key|LeftMouseButton`
  (params (Key :type "Key Structure"))
  (:`Pressed`
    (bind _outactors (`GameplayStatics.GetAllActorsOfClass` "/Game/Ship/Helicopter.Helicopter_C"))
    (if (> (`KismetArrayLibrary.Array_Length` _outactors) 0)
      (`/Game/Ship/Helicopter.Fire` (`|GetArrayItem` _outactors))))
  (:`Released`
    (cast `/Game/Blueprints/CoordinatePlane` (`.HitActor` (`GameplayStatics.BreakHitResult` (`self.GetHitResultUnderCursorForObjects` (`|MakeArray` "ObjectTypeQuery1" "ObjectTypeQuery2" :!type "EObjectTypeQuery Enum") false))))
    (set `self.ChangingSetpoint` false)))

(event `Key|RightMouseButton`
  (params (Key :type "Key Structure"))
  (:`Pressed`
    (bind _outactors (`GameplayStatics.GetAllActorsOfClass` "/Game/Ship/Helicopter.Helicopter_C"))
    (if (> (`KismetArrayLibrary.Array_Length` _outactors) 0)
      (`/Game/Ship/Helicopter.FireMachineGun` (`|GetArrayItem` _outactors) true)))
  (:`Released`
    (bind _outactors_2 (`GameplayStatics.GetAllActorsOfClass` "/Game/Ship/Helicopter.Helicopter_C"))
    (if (> (`KismetArrayLibrary.Array_Length` _outactors_2) 0)
      (`/Game/Ship/Helicopter.FireMachineGun` (`|GetArrayItem` _outactors_2) false))))

(event `Key|Two`
  (params (Key :type "Key Structure"))
  (:`Pressed`
    (bind _outactors (`GameplayStatics.GetAllActorsOfClass` "/Game/Ship/Helicopter.Helicopter_C"))
    (if (> (`KismetArrayLibrary.Array_Length` _outactors) 0)
      (`/Game/Ship/Helicopter.Repair25` (`|GetArrayItem` _outactors)))))

(event `Key|Zero`
  (params (Key :type "Key Structure"))
  (:`Pressed`
    (bind _outactors (`GameplayStatics.GetAllActorsOfClass` "/Game/Ship/Helicopter.Helicopter_C"))
    (if (> (`KismetArrayLibrary.Array_Length` _outactors) 0)
      (bind _output (`|GetArrayItem` _outactors))
      (set `/Game/Ship/Helicopter.Damage` (`/Game/Ship/Helicopter.MaxHealth` _output) _output))))

(event `Key|Nine`
  (params (Key :type "Key Structure"))
  (:`Pressed`
    (bind _outactors (`GameplayStatics.GetAllActorsOfClass` "/Game/Ship/Helicopter.Helicopter_C"))
    (if (> (`KismetArrayLibrary.Array_Length` _outactors) 0)
      (`GameplayStatics.ApplyDamage` (`|GetArrayItem` _outactors) 100.0))))

(event `Key|One`
  (params (Key :type "Key Structure"))
  (bind _rocketscost (`self.RocketsCost`))
  (:`Pressed`
    (bind _ashelicopter_hud (cast `/Game/Ship/HUD/HelicopterHUD` (`self.GetHUD`)))
    (bind _hudwidget (`/Game/Ship/HUD/HelicopterHUD.HUDWidget` _ashelicopter_hud))
    (bind _coinscount (`/Game/Ship/HUD/HelicopterHUDWidget.CoinsCount` _hudwidget))
    (if (>= _coinscount _rocketscost)
      (set `/Game/Ship/HUD/HelicopterHUDWidget.CoinsCount` (- _coinscount _rocketscost) _hudwidget)
      (bind _outactors (`GameplayStatics.GetAllActorsOfClass` "/Game/Ship/Helicopter.Helicopter_C"))
      (if (> (`KismetArrayLibrary.Array_Length` _outactors) 0)
        (bind _output (`|GetArrayItem` _outactors))
        (set `/Game/Ship/Helicopter.Rockets` (+ (`/Game/Ship/Helicopter.Rockets` _output) 100) _output)))))

(fn `GetSelectedActor`
  (returns (Actor :type "Actor Object Reference"))
  (return (`/Game/Blueprints/PIDHUD.GetSelectedActor` (`self.HUD`))))

(fn `SelectActor`
  (params (Actor :type "Actor Object Reference"))
  (`/Game/Blueprints/PIDHUD.SelectActor` (`self.HUD`) Actor))

(fn `UserConstructionScript`)