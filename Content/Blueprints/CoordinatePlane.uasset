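; CoordinatePlane is a clickable actor that converts mouse clicks on it into 2D coordinates.
; On click, it traces WorldStatic objects under the cursor and, if it is the hit actor, broadcasts Clicked with the world hit location's Y and Z divided by 100.
; Every Tick, a helper function draws green debug number labels at 100-unit intervals along the Z axis.
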(event `self.ReceiveTick`
  (params (DeltaSeconds :type "Float (single-precision)"))
  (`self.NewFunction_0`))

(event `self.ReceiveActorOnClicked`
  (params (ButtonPressed :type "Key Structure"))
  (bind (_bblockinghit _binitialoverlap _time _distance _location _impactpoint _normal _impactnormal _physmat _hitactor) (`GameplayStatics.BreakHitResult` (`PlayerController.GetHitResultUnderCursorForObjects` (`GameplayStatics.GetPlayerController` 0) (`|MakeArray` "ObjectTypeQuery1" :!type "EObjectTypeQuery Enum") false)))
  (if (== _hitactor self)
    (`self.Clicked` (`KismetMathLibrary.MakeVector2D` (.y (/ _location 100.0)) (.z (/ _location 100.0))))))

(fn `NewFunction_0`
  (for _index (range 101)
    (`KismetSystemLibrary.DrawDebugString` (`KismetMathLibrary.MakeVector` 0.0 0.0 (* _index 100.0)) (`KismetStringLibrary.Conv_IntToString` _index) null (struct :`G` 1.0 :`B` 0.041685 :`A` 1.0))))

(fn `UserConstructionScript`)