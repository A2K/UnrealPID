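; PIDHUD is the HUD actor that owns the PID widget and exposes it to the rest of the game.
; On BeginPlay it creates the widget, adds it to the viewport and registers itself on the PIDPlayerController.
; Its functions forward the PID component, actor selection and setpoint to the widget, and return the owner of the widget's current PID component as the selected actor.
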(event `self.ReceiveBeginPlay`
  (bind _returnvalue (`GameplayStatics.GetPlayerController` 0))
  (bind _returnvalue_2 (`|CreateWidget` "/Game/PIDWidget.PIDWidget_C" _returnvalue))
  (`|ExecutionSequence`
    (:`then_0`
      (bind _output_get (set `self.PIDWidget` _returnvalue_2))
      (`UserWidget.AddToViewport` _output_get 0))
    (:`then_1`
      (bind _aspidplayer_controller (cast `/Game/Blueprints/PIDPlayerController` _returnvalue))
      (set `/Game/Blueprints/PIDPlayerController.HUD` self _aspidplayer_controller))))

(fn `GetSelectedActor`
  (returns (Actor :type "Actor Object Reference"))
  (bind _pid (`/Game/PIDWidget.PID` (`self.PIDWidget`)))
  (`/Engine/EditorBlueprintResources/StandardMacros.IsValid` _pid
    (:`Is Valid`
      (return (`ActorComponent.GetOwner` _pid)))
    (:`Is Not Valid`
      (return null))))

(fn `SelectActor`
  (params (Actor :type "Actor Object Reference"))
  (`/Game/PIDWidget.SelectActor` (`self.PIDWidget`) Actor))

(fn `SetPIDComponent`
  (params (PID :type "/Game/PID Object Reference"))
  (set `/Game/PIDWidget.PID` PID (`self.PIDWidget`)))

(fn `SetSetpoint`
  (params (Setpoint :type "Float (double-precision)"))
  (`/Game/PIDWidget.SetSetpoint` (`self.PIDWidget`) Setpoint))

(fn `UserConstructionScript`)